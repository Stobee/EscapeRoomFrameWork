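; BP_MainHUD is the HUD Blueprint that manages the FPS screen and the close-up inspect mode UI.
; On BeginPlay it creates both widgets, with the inspect screen hidden on a higher Z-order.
; VisibleInspectModeWidget shows that screen, enables a locked cursor with Game and UI input, and swaps IMC_Default for IMC_InspectMode so only inspect controls apply.
; DismissInspectModeWidget restores the default mapping, hides the widget and cursor, and returns to Game Only input.
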(event `self.ReceiveBeginPlay`
  (set `self.PlayerControllerRef` (`GameplayStatics.GetPlayerController` 0))
  (bind _returnvalue (`|CreateWidget` "/Game/Widgets/WBP_FPSModeScreen.WBP_FPSModeScreen_C"))
  (`UserWidget.AddToViewport` _returnvalue 0)
  (bind _returnvalue_2 (`|CreateWidget` "/Game/Widgets/WBP_InvestigateModeScreen.WBP_InvestigateModeScreen_C"))
  (set `self.WBPInspectModeRef` _returnvalue_2)
  (`Widget.SetVisibility` _returnvalue_2 "Hidden")
  (`UserWidget.AddToViewport` _returnvalue_2 10))

(fn `DismissInspectModeWidget`
  (bind _returnvalue (pcsubsystem `EnhancedInputLocalPlayerSubsystem` (`self.PlayerControllerRef`)))
  ; IMC 다시 디폴트로 바꾸고 위젯 숨긴 뒤에 커서 끔
  (`EnhancedInputSubsystemInterface.RemoveMappingContext` _returnvalue "/Game/Input/IMC_InspectMode.IMC_InspectMode" (struct))
  (`EnhancedInputSubsystemInterface.AddMappingContext` _returnvalue "/Game/Input/IMC_Default.IMC_Default" 0 (struct))
  (`Widget.SetVisibility` (`self.WBPInspectModeRef`) "Hidden")
  (set `PlayerController.bShowMouseCursor` false (`self.PlayerControllerRef`))
  (`WidgetBlueprintLibrary.SetInputMode_GameOnly` (`self.PlayerControllerRef`)))

(fn `UserConstructionScript`)

(fn `VisibleInspectModeWidget`
  (bind _returnvalue (pcsubsystem `EnhancedInputLocalPlayerSubsystem` (`self.PlayerControllerRef`)))
  ; 위젯 보여주고, IMC 변경해서 밀착 조사 모드 전용 조작만 하게 만듦
  (`Widget.SetVisibility` (`self.WBPInspectModeRef`) "Visible")
  (set `PlayerController.bShowMouseCursor` true (`self.PlayerControllerRef`))
  (`WidgetBlueprintLibrary.SetInputMode_GameAndUIEx` (`self.PlayerControllerRef`) (`self.WBPInspectModeRef`) "LockAlways" false)
  (`EnhancedInputSubsystemInterface.RemoveMappingContext` _returnvalue "/Game/Input/IMC_Default.IMC_Default" (struct))
  (`EnhancedInputSubsystemInterface.AddMappingContext` _returnvalue "/Game/Input/IMC_InspectMode.IMC_InspectMode" 1 (struct)))