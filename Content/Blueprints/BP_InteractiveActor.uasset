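; Data-driven interactable actor whose meshes and action (door, drawer, read hint, pick up item, investigate) come from its DT_Actors row.
; Construction sets the meshes; BeginPlay caches row data and initializes the prompt widget, which is toggled with a custom-depth outline.
; SelectAct dispatches by enum: doors and drawers move Pivot via FlipFlop timelines, investigation calls the character's inspect mode.
; Items and hints go to the inventory interface and HUD, then destroy the actor.
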(event `self.ReceiveBeginPlay`
  ; 데이터 테이블 캐싱하고, 해당 정보로 위젯 초기화
  (`self.DataTableCach` (`self.ActorRowName`))
  (`self.InitWidgetText`))

(event `/Game/Blueprints/Interfaces/BPI_InteractiveActorInterface.SelectInteractiveAct`
  ; 상호작용 결정함
  (`self.SelectAct` (`self.Interactive Act`)))

(event `/Game/Blueprints/Interfaces/BPI_InteractiveActorInterface.DoorOpenAndClose`
  ; 문 열고 닫는 로직 (테스트 중)
  (bind _isa (`/Engine/EditorBlueprintResources/StandardMacros.FlipFlop`)
    (:`A`
      (bind (_direction _newtrack_0) (`Timeline|DoorTimeline` :!via `PlayFromStart` :!label _label)
        (:`Update`
          (`SceneComponent.K2_SetRelativeRotation` (`self.Pivot`) (`KismetMathLibrary.MakeRotator` 0.0 (`KismetMathLibrary.Lerp` 0.0 90.0 _newtrack_0)) false false))
        (:`Finished`
          (bind _output_get (set `self.bIsOpened` _isa))
          (`/Game/Widgets/WBP_InteractiveInfo.UpdateText` (`self.WBPInteractiveInfoRef`) (`self.Interactive Act`) _output_get))))
    (:`B`
      (goto _label :!via `ReverseFromEnd`))))

(event `/Game/Blueprints/Interfaces/BPI_InteractiveActorInterface.SlideOpenAndClose`
  ; 서랍 열고 닫는 로직 (테스트 중)
  (bind _isa (`/Engine/EditorBlueprintResources/StandardMacros.FlipFlop`)
    (:`A`
      (bind (_direction _newtrack_0) (`Timeline|DrawerTimeline` :!via `PlayFromStart` :!label _label_2)
        (:`Update`
          (`SceneComponent.K2_SetRelativeLocation` (`self.Pivot`) (`KismetMathLibrary.MakeVector` (`KismetMathLibrary.Lerp` 0.0 (* (.x (`StaticMeshComponent.GetLocalBounds` (`self.MovableStaticMesh`))) 0.7) _newtrack_0)) false false))
        (:`Finished`
          (bind _output_get (set `self.bIsOpened` _isa))
          (`/Game/Widgets/WBP_InteractiveInfo.UpdateText` (`self.WBPInteractiveInfoRef`) (`self.Interactive Act`) _output_get))))
    (:`B`
      (goto _label_2 :!via `ReverseFromEnd`))))

(event `/Game/Blueprints/Interfaces/BPI_InteractiveActorInterface.ItemPickUp`
  ; 아이템 줍고 인벤토리에 저장
  (`self.ItemPickUpAndSave` (`self.Out Row Item ID`)))

(event `/Game/Blueprints/Interfaces/BPI_InteractiveActorInterface.ShowInteractionInfo`
  ; 라인트레이스에 따라 위젯 컴포넌트 visible, 메쉬 outline 켜고 끄기
  (`SceneComponent.SetVisibility` (`self.InteractWidget`) true false)
  (`PrimitiveComponent.SetRenderCustomDepth` (`self.BaseStaticMesh`) true))

(event `/Game/Blueprints/Interfaces/BPI_InteractiveActorInterface.DismissInteractionInfo`
  ; 라인트레이스에 따라 위젯 컴포넌트 visible, 메쉬 outline 켜고 끄기
  (`SceneComponent.SetVisibility` (`self.InteractWidget`) false false)
  (`PrimitiveComponent.SetRenderCustomDepth` (`self.BaseStaticMesh`) false))

(event `/Game/Blueprints/Interfaces/BPI_InteractiveActorInterface.ShowHintWidgetAndSaveInventory`
  ; 단서 주워서 위젯 띄우고 인벤토리에 저장
  (`self.ShowHintWidget` (`self.Out Row Hint ID`)))

(event `/Game/Blueprints/Interfaces/BPI_InteractiveActorInterface.SetTransform`
  (params (NewTransform :type "Transform Structure"))
  ; 액터 트랜스폼 변경
  (`self.K2_SetActorTransform` NewTransform))

(fn `DataTableCach`
  (params (RowName :type Name))
  ; 메쉬를 제외한 액터에 필요한 모든 정보 캐싱
  (set `self.PlayerCharacterRef` (`GameplayStatics.GetPlayerCharacter` 0))
  (set `self.PlayerControllerRef` (`GameplayStatics.GetPlayerController` 0))
  (set `self.HUDRef` (`PlayerController.GetHUD` (`self.PlayerControllerRef`)))
  (bind _returnvalue (`|GetDataTableRow` "/Game/Datas/DataTables/DT_Actors.DT_Actors" RowName)
    (:`then`
      (set `self.ActorTransform` (`.ActorTransform_28_AB2A99324CE0A39365B6A89FCAFB7D15` (break `/Game/Datas/Structures/ST_Actor` _returnvalue)))
      (bind _output_get (set `self.Interactive Act` (`.InteractiveAct_35_DEBA613A478E1367198D3DA70B6499CB` (break `/Game/Datas/Structures/ST_Actor` _returnvalue))))
      (set `self.Out Row Use Item` (`.bUseItem_33_40449EAD4F15D99EF0B6B4A1DA88B955` (break `/Game/Datas/Structures/ST_Actor` _returnvalue)))
      (if (`|EnumEquality` _output_get "NewEnumerator2")
        (set `self.Out Row Hint ID` (`.Hint_ID_47_FB61FE6A4753B2F4315B0F9895F05F7B` (break `/Game/Datas/Structures/ST_Actor` _returnvalue)))
        (elif (`|EnumEquality` _output_get "NewEnumerator5")
          (set `self.Out Row Item ID` (`.Item_ID_46_F8BF3B3D4529021C05D55394B12EFBA9` (break `/Game/Datas/Structures/ST_Actor` _returnvalue)))))
      (if (!= (`.LevelEndFlag_20_CDE0C8A948F8604985560DBDB53F33E8` (break `/Game/Datas/Structures/ST_Actor` _returnvalue)) "None")
        ; LevelEnd 로직 예정
        (set `self.Level End Flag` (`.LevelEndFlag_20_CDE0C8A948F8604985560DBDB53F33E8` (break `/Game/Datas/Structures/ST_Actor` _returnvalue)))
        (else
          (return))))))

(fn `InitWidgetText`
  ; 위젯 텍스트 초기화
  (bind _aswbp_interactive_info (cast `/Game/Widgets/WBP_InteractiveInfo` (`WidgetComponent.GetUserWidgetObject` (`self.InteractWidget`))))
  (bind _output_get (set `self.WBPInteractiveInfoRef` _aswbp_interactive_info))
  (`/Game/Widgets/WBP_InteractiveInfo.UpdateText` _output_get (`self.Interactive Act`) (`self.bIsOpened`)))

(fn `ItemPickUpAndSave`
  (params (ItemID :type Name))
  (bind _returnvalue (`self.GetComponentsByInterface` (`self.PlayerCharacterRef`) "/Game/Blueprints/Interfaces/BPI_InventoryInterface.BPI_InventoryInterface_C"))
  ; 아이템 액터와 상호작용 해서 아이템 ID를 인벤토리에 저장 후 액터 삭제
  (if (not (<= (`KismetArrayLibrary.Array_Length` _returnvalue) 0))
    (message `/Game/Blueprints/Interfaces/BPI_InventoryInterface.AddItem` (`|GetArrayItem` _returnvalue) ItemID)
    (message `/Game/Blueprints/Interfaces/BPI_HUDWidgetControl.UpdateItemInventoryWidget` (`self.HUDRef`) (`local.ItemID`))
    (`self.K2_DestroyActor`)))

(fn `SelectAct`
  (params (Selection :type "/Game/Datas/Enums/E_InteractiveActs Enum" :default "NewEnumerator0"))
  ; 해당 enum값에 따라 다른 상호작용 실행
  (switch `/Game/Datas/Enums/E_InteractiveActs` Selection
    (:`NewEnumerator0`
      (`self.DoorOpenAndClose`))
    (:`NewEnumerator3`
      (`self.SlideOpenAndClose`))
    (:`NewEnumerator2`
      (`self.ShowHintWidgetAndSaveInventory`))
    (:`NewEnumerator4`
      (`self.StartInspectMode`))
    (:`NewEnumerator5`
      (`self.ItemPickUp`))))

(fn `ShowHintWidget`
  (params (HintID :type Name))
  (bind _returnvalue (`self.GetComponentsByInterface` (`self.PlayerCharacterRef`) "/Game/Blueprints/Interfaces/BPI_InventoryInterface.BPI_InventoryInterface_C"))
  ; 힌트 액터와 상호작용하여 힌트 위젯 보여주고, 플레이어 인벤토리에 힌트 ID 저장 후 액터 삭제
  (message `/Game/Blueprints/Interfaces/BPI_HUDWidgetControl.HintTextWidgetVisible` (`self.HUDRef`) (`local.HintID`))
  (if (not (<= (`KismetArrayLibrary.Array_Length` _returnvalue) 0))
    (message `/Game/Blueprints/Interfaces/BPI_InventoryInterface.AddHint` (`|GetArrayItem` _returnvalue) (`local.HintID`))
    (set `PlayerController.bShowMouseCursor` true (`self.PlayerControllerRef`))
    (`WidgetBlueprintLibrary.SetInputMode_UIOnlyEx` (`self.PlayerControllerRef`) null "LockAlways")
    (message `/Game/Blueprints/Interfaces/BPI_HUDWidgetControl.UpdateHintInventoryWidget` (`self.HUDRef`) (`self.Out Row Hint ID`))
    (`self.K2_DestroyActor`)))

(fn `StartInspectMode`
  ; 캐릭터에게 자신의 정보를 보내고 밀착 조사 모드 시작 호출
  (message `/Game/Blueprints/Interfaces/BPI_InpectModeInterface.StartInspectMode` (`self.PlayerCharacterRef`) self (`self.GetTransform` self)))

(fn `UserConstructionScript`
  (locals (DoorOrDrawer :type "/Game/Datas/Enums/E_InteractiveActs Enum" :default "NewEnumerator0"))
  (bind _movablestaticmesh (`self.MovableStaticMesh`))
  ; 메쉬 정보를 먼저 가져옴. MovableMesh는 있을 경우에만 가져옴.
  (bind _returnvalue (`|GetDataTableRow` "/Game/Datas/DataTables/DT_Actors.DT_Actors" (`self.ActorRowName`))
    (:`then`
      (`StaticMeshComponent.SetStaticMesh` (`self.BaseStaticMesh`) (`.ActorBaseMesh_22_82E90662408960C2757F9C814DD00CCA` (break `/Game/Datas/Structures/ST_Actor` _returnvalue)))
      (`/Engine/EditorBlueprintResources/StandardMacros.IsValid` (`.ActorMovableMesh_24_F5FCB40640D9ED74B67D289697AADA74` (break `/Game/Datas/Structures/ST_Actor` _returnvalue))
        (:`Is Valid`
          (`StaticMeshComponent.SetStaticMesh` (`self.MovableStaticMesh`) (`.ActorMovableMesh_24_F5FCB40640D9ED74B67D289697AADA74` (break `/Game/Datas/Structures/ST_Actor` _returnvalue)))
          (set `local.DoorOrDrawer` (`.InteractiveAct_35_DEBA613A478E1367198D3DA70B6499CB` (break `/Game/Datas/Structures/ST_Actor` _returnvalue)))
          (switch `/Game/Datas/Enums/E_InteractiveActs` (`local.DoorOrDrawer`)
            (:`NewEnumerator3`
              (`SceneComponent.K2_SetRelativeLocation` _movablestaticmesh (`KismetMathLibrary.MakeVector` (.x (`StaticMeshComponent.GetLocalBounds` _movablestaticmesh))) false false))))))))